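; Player character for a melee action game, with Enhanced Input movement and look, sprint, roll, light and heavy attacks, and an E-key combo montage.
; Sprint, roll and attacks drain a shared stamina pool that Tick regenerates after a delay.
; Attack montage notifies toggle visibility of the BoxPAttack hitbox.
; Capsule overlap with the enemy's box deals damage once (CanDomm never resets), updates the widget and plays hit or death montages.
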(event OnComponentBeginOverlap(CapsuleComponent)
  (params (OverlappedComponent :type Primitive%20Component%20Object%20Reference) (OtherActor :type Actor%20Object%20Reference) (OtherComp :type Primitive%20Component%20Object%20Reference) (OtherBodyIndex :type Integer) (bFromSweep :type Boolean) (SweepResult :type Hit%20Result%20Structure%20%28by%20ref%29))
  (bind _mesh (Variables|Character|GetMesh))
  (if (Variables|Default|GetCanDomm)
    (if (== OtherActor (Variables|/Game/BS_Ennemis.BS_Ennemis_C|GetBox (Variables|Default|GetEnnemis_Ref)))
      (bind _output_get (Variables|Default|SetHealthPLayer (- (Variables|Default|GetHealthPLayer) 1e+02)))
      (Default|PlayerDegat (Variables|Default|GetWidget_ref) _output_get)
      (Variables|Default|SetCanDomm false)
      (if (<= (Variables|Default|GetHealthPLayer) 0.0)
        (bind _notifyname (Animation|Montage|PlayMontage _mesh "/Game/Sword_Animations/Animations/Sequence1/08_Hit/06_Hit_Large_Combat/Montage_MortEnnmis.Montage_MortEnnmis")
          (:OnNotifyBegin
            (if (== _notifyname "DeathEnnemis")
              (Actor|DestroyActor))))
        (else
          (bind _notifyname_2 (Animation|Montage|PlayMontage _mesh "/Game/Sword_Animations/Animations/Sequence1/08_Hit/02_Hit_Combat/HitEnnemis.HitEnnemis")
            (:OnNotifyBegin
              (if (== _notifyname_2 "Hit_Domm")
                _))))))))

(event Input|EnhancedActionEvents|EnhancedInputActionIA_Move
  (params (ActionValue :type Vector%202D%20Structure) (ElapsedSeconds :type Float%20%28double-precision%29) (TriggeredSeconds :type Float%20%28double-precision%29) (InputAction :type Input%20Action%20Object%20Reference :default "/Game/Inputs/Actions/IA_Move.IA_Move"))
  (bind _camera (Variables|Default|GetCamera))
  (bind _returnvalue (Transformation|GetWorldRotation _camera))
  (if (Variables|Default|GetCanMove)
    (Pawn|Input|AddMovementInput (Math|Vector|GetForwardVector (Math|Rotator|MakeRotator 0.0 0.0 (.yaw _returnvalue))) (.x ActionValue) false)
    (Pawn|Input|AddMovementInput (Math|Vector|GetRightVector (Math|Rotator|MakeRotator 0.0 0.0 (.yaw _returnvalue))) (.y ActionValue) false)))

(event Input|EnhancedActionEvents|EnhancedInputActionIA_Look
  (params (ActionValue :type Vector%202D%20Structure) (ElapsedSeconds :type Float%20%28double-precision%29) (TriggeredSeconds :type Float%20%28double-precision%29) (InputAction :type Input%20Action%20Object%20Reference :default "/Game/Inputs/Actions/IA_Look.IA_Look"))
  (Pawn|Input|AddControllerYawInput (.x ActionValue))
  (Pawn|Input|AddControllerPitchInput (.y ActionValue)))

(event EventBeginPlay
  (bind _asplayer_controller (Utilities|Casting|CastToPlayerController (Pawn|GetController)))
  (Input|AddMappingContext (PlayerController|LocalPlayerSubsystems|GetEnhancedInputLocalPlayerSubsystem _asplayer_controller) "/Game/Inputs/IMC_Player.IMC_Player" 0 "(bIgnoreAllPressedKeysUntilRelease=True,bForceImmediately=False,bNotifyUserSettings=False)")
  (Variables|Default|SetHealthPLayer 1e+02)
  (Variables|Default|SetStamina 1e+02)
  (bind _returnvalue (UserInterface|CreateWidget "/Game/Widget_BP_Player.Widget_BP_Player_C" (Variables|Default|GetSelfPlayer)))
  (UserInterface|Viewport|AddtoPlayerScreen _returnvalue))

(event EventTick
  (params (DeltaSeconds :type Float%20%28single-precision%29))
  (Development|PrintString (Utilities|String|ToString(Float) (Variables|Default|GetStamina)) true true "(R=0.000000,G=0.660000,B=1.000000,A=1.000000)" 0.25)
  (if (Variables|Default|GetCanregStam)
    (if (not (> (Variables|Default|GetStamina) 1e+02))
      (Variables|Default|SetStamina (+ (Variables|Default|GetStamina) 0.5)))
    (elif (Variables|Default|GetSprint)
      (if (> (Variables|Default|GetStamina) 0.0)
        (bind _output_get (Variables|Default|SetStamina (- (Variables|Default|GetStamina) 0.5)))
        (Default|Stamina (Variables|Default|GetWidget_ref) _output_get))
      (else
        (Utilities|FlowControl|Delay 3.5)
        (Variables|Default|SetCanregStam true)))))

(event Input|KeyboardEvents|SpaceBar
  (params (Key :type Key%20Structure :default "None"))
  (:Pressed
    (if (Variables|Default|GetRoll)
      (Variables|Default|SetRoll false)
      (if (> (Variables|Default|GetStamina) 0.0)
        (Variables|Default|SetCanregStam false)
        (bind _output_get (Variables|Default|SetStamina (- (Variables|Default|GetStamina) 2e+01)))
        (Default|Stamina (Variables|Default|GetWidget_ref) _output_get)
        (Animation|Montage|PlayMontage (Variables|Character|GetMesh) "/Game/Sword_Animations/Animations/Sequence1/07_Roll/02_Roll_Combat/M_Roll.M_Roll"
          (:then
            (Utilities|FlowControl|Delay 1.5)
            (Variables|Default|SetRoll true)))))))

(event Input|KeyboardEvents|LeftShift
  (params (Key :type Key%20Structure :default "None"))
  (bind _charactermovement (Variables|Character|GetCharacterMovement))
  (bind _charactermovement_2 (Variables|Character|GetCharacterMovement))
  (:Pressed
    (if (> (Variables|Default|GetStamina) 0.0)
      (Variables|Default|SetSprint true)
      (Variables|Default|SetCanregStam false)
      (Variables|/Script/Engine.CharacterMovementComponent|SetMaxWalkSpeed _charactermovement_2 9e+02)
      (Variables|/Script/Engine.CharacterMovementComponent|SetbUseControllerDesiredRotation _charactermovement_2 false)
      (Variables|/Script/Engine.CharacterMovementComponent|SetbOrientRotationToMovement _charactermovement_2 true)))
  (:Released
    (Variables|Default|SetSprint false)
    (Variables|/Script/Engine.CharacterMovementComponent|SetMaxWalkSpeed _charactermovement 6e+02)
    (Variables|/Script/Engine.CharacterMovementComponent|SetbUseControllerDesiredRotation _charactermovement true)
    (Variables|/Script/Engine.CharacterMovementComponent|SetbOrientRotationToMovement _charactermovement false)
    (Utilities|FlowControl|Delay 1.5)))

(event Input|KeyboardEvents|E
  (params (Key :type Key%20Structure :default "None"))
  (:Pressed
    (Animation|Montage|PlayMontage (Variables|Character|GetMesh) "/Game/Sword_Animations/Animations/Sequence1/02_Attack/03_Combo_Attack_03/Combo_Attack_03_01_Seq_Montage.Combo_Attack_03_01_Seq_Montage"))
  (:Released
    (Animation|Montage|PlayMontage (Variables|Character|GetMesh) "/Game/Sword_Animations/Animations/Sequence1/02_Attack/03_Combo_Attack_03/Combo_Attack_03_01_Seq_Montage.Combo_Attack_03_01_Seq_Montage" 1.0 0.0 "EndHold")))

(event Input|MouseEvents|LeftMouseButton
  (params (Key :type Key%20Structure :default "None"))
  (bind _box_p_attack (Variables|Default|GetBox_P_Attack))
  ;[1 1 1] Attaque legere
  (:Pressed
    (if (Variables|Default|GetAttackBas)
      (Variables|Default|SetAttackBas false)
      (if (> (Variables|Default|GetStamina) 0.0)
        (Variables|Default|SetCanregStam false)
        (bind _output_get (Variables|Default|SetStamina (- (Variables|Default|GetStamina) 15.0)))
        (Default|Stamina (Variables|Default|GetWidget_ref) _output_get)
        (bind _notifyname (Animation|Montage|PlayMontage (Variables|Character|GetMesh) "/Game/Sword_Animations/Animations/Sequence1/02_Attack/04_Combo_Attack_04/M_AttackBas.M_AttackBas")
          (:then
            (Utilities|FlowControl|Delay 2.0)
            (Variables|Default|SetAttackBas true))
          (:OnNotifyBegin
            (if (== _notifyname "Hit_Attack_Leg")
              (Rendering|SetVisibility _box_p_attack true false)))
          (:OnNotifyEnd
            (if (== _notifyname "Hit_Attack_Leg")
              (Rendering|SetVisibility _box_p_attack false false))))))))

(event Input|MouseEvents|RightMouseButton
  (params (Key :type Key%20Structure :default "None"))
  (bind _box_p_attack (Variables|Default|GetBox_P_Attack))
  ;[1 1 1] Attaque Lourde
  (:Pressed
    (if (Variables|Default|GetAttackBas)
      (Variables|Default|SetAttackBas false)
      (if (> (Variables|Default|GetStamina) 0.0)
        (Variables|Default|SetCanregStam false)
        (if (not (< (- (Variables|Default|GetStamina) 3e+01) 0.0))
          (bind _output_get (Variables|Default|SetStamina (- (Variables|Default|GetStamina) 3e+01)))
          (Default|Stamina (Variables|Default|GetWidget_ref) _output_get)
          (bind _notifyname (Animation|Montage|PlayMontage (Variables|Character|GetMesh) "/Game/Sword_Animations/Animations/Sequence1/02_Attack/12_Run_Attact/M_AttackLourde.M_AttackLourde")
            (:then
              (Utilities|FlowControl|Delay 2.5)
              (Variables|Default|SetAttackBas true))
            (:OnNotifyBegin
              (if (== _notifyname "Hit_A_Lourde")
                (Rendering|SetVisibility _box_p_attack true false)))
            (:OnNotifyEnd
              (if (== _notifyname "Hit_A_Lourde")
                (Rendering|SetVisibility _box_p_attack false false)))))))))

(fn ConstructionScript)